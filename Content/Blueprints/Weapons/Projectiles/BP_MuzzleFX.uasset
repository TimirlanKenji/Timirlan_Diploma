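; Short-lived muzzle flash effect actor that animates a mesh and point light, then destroys itself.
; On BeginPlay the static mesh's world scale is randomized per axis to vary each flash.
; The Muzzle timeline's ScaleA curve then drives both mesh scale and light intensity through tuning multipliers.
; A one-second timer destroys the actor.
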(event EventBeginPlay
  (Utilities|FlowControl|Sequence
    (:then_0
      (Variables|Default|SetMuzzleScale (CallFunction|RndVector (Transformation|GetWorldScale (Variables|Default|GetStaticMesh))))
      (bind _scalea (Timeline|Muzzle Play)
        (:Update
          (Utilities|FlowControl|Sequence
            (:then_0
              (Transformation|SetWorldScale3D (Variables|Default|GetStaticMesh) (* (Variables|Default|GetMuzzleScale) (* _scalea (Variables|Default|GetMuzzleScaleKoef)))))
            (:then_1
              (Rendering|Components|Light|SetIntensity (Variables|Default|GetPointLight) (* _scalea (Variables|Default|GetLightKoef))))))))
    (:then_1
      (Utilities|Time|SetTimerbyFunctionName 0 "ReadyToDestroy" 1.0))))

(event Collision|EventActorBeginOverlap
  (params (OtherActor :type Actor%20Object%20Reference)))

(event EventTick
  (params (DeltaSeconds :type Float%20%28single-precision%29)))

(fn ConstructionScript)

(fn RndVector
  (params (InVec :type Vector))
  (bind (_x _y _z) (Math|Vector|BreakVector InVec))
  (return (Math|Vector|MakeVector (* (Math|Random|RandomFloatinRange 0.8 1.2) _x) (* (Math|Random|RandomFloatinRange 0.8 1.2) _y) (* (Math|Random|RandomFloatinRange 0.8 1.2) _z))))

(fn ReadytoDestroy
  (Actor|DestroyActor))