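; Base weapon actor that configures itself from a DT_Weapons row, scaling damage by the owning character's multiplier.
; While active, Tick polls fire input and weapon state to spawn type-specific projectiles with muzzle FX and sound.
; Timers gate shot delay and reload, which draws on reserve ammo, while status changes are broadcast.
; A line trace drives a laser sight's length and dot light, and activation toggles mesh visibility and that light.
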(event EventBeginPlay
  (|CallParentFunction) ; This node is disabled and will not be called.\nDrag off pins to build functionality.
)

(event Collision|EventActorBeginOverlap
  (params (OtherActor :type Actor%20Object%20Reference))
  (|CallParentFunction OtherActor) ; This node is disabled and will not be called.\nDrag off pins to build functionality.
)

(event EventTick
  (params (DeltaSeconds :type Float%20%28single-precision%29))
  (|CallParentFunction DeltaSeconds)
  (if (Variables|Configure|GetIsWeaponActive)
    (Shoot|Shooting)
    (CallFunction|AimUpdate)))

(fn ConstructionScript
  (|CallParentFunction))

(fn ShootInputRecived
  (params (InProcess :type Boolean))
  (Variables|Shoot|SetInProcess InProcess))

(fn Shooting
  ;[1 1 1] Check allow to shoot
  (if (and (Variables|Shoot|GetInProcess) (Utilities|Enum|Equal(Enum) (Variables|Default|GetWeaponState) "NewEnumerator0"))
    (Shoot|SingleShot)
    (bind _allowshooting (Reload|RoundsCount))
    (if _allowshooting
      (Utilities|Time|SetTimerbyEvent (EventDispatchers|CreateEvent :!event AfterShotDelayEnd) (Variables|Shoot|GetAfterShotDelay))
      (Variables|Default|SetWeaponState "NewEnumerator4")
      (Default|CallOnWeaponStatusChanged)
      (else
        (Variables|Default|SetWeaponState "NewEnumerator1")
        (if (Variables|Reload|GetIsAutoReloading)
          (Reload|Reload)
          (else
            (Default|CallOnWeaponStatusChanged)))))))

(fn SingleShot
  (bind _returnvalue (Game|SpawnActorfromClass (Utilities|Select :Index (Variables|Configure|GetCurrenWeaponType) :NewEnumerator0 "/Game/Blueprints/Weapons/Projectiles/BP_BaseProjectile_PistolBullet.BP_BaseProjectile_PistolBullet_C" :NewEnumerator1 "/Game/Blueprints/Weapons/Projectiles/BP_BaseProjectile_RifleBullet.BP_BaseProjectile_RifleBullet_C" :NewEnumerator2 "/Game/Blueprints/Weapons/Projectiles/BP_BaseProjectile_ShotgunBullet.BP_BaseProjectile_ShotgunBullet_C" :NewEnumerator3 "/Game/Blueprints/Weapons/Projectiles/BP_BaseProjectile_Rocket.BP_BaseProjectile_Rocket_C") (Transformation|GetWorldTransform (Variables|Default|GetMuzzle)) "Undefined" 0 0))
  (bind _asbp_base_projectile (Utilities|Casting|CastToBP_BaseProjectile _returnvalue))
  ;[1 1 1] Add Damage to Proj
  (Default|AddDamage _asbp_base_projectile (Variables|Configure|GetCurrentDamage))
  (Audio|Components|Audio|Play (Variables|Default|GetShotSound) 0.0)
  (bind _returnvalue_2 (Game|SpawnActorfromClass "/Game/Blueprints/Weapons/Projectiles/BP_MuzzleFX.BP_MuzzleFX_C" (Transformation|GetWorldTransform (Variables|Default|GetMuzzle)) "Undefined" 0 0))
  (Transformation|AttachComponentToComponent _returnvalue_2 (Variables|Default|GetMuzzle) "None" "SnapToTarget" "SnapToTarget" "SnapToTarget" true))

(fn AfterShotDelayEnd
  (Variables|Default|SetWeaponState "NewEnumerator0"))

(fn Reload
  (Variables|Default|SetWeaponState "NewEnumerator2")
  (Audio|Components|Audio|Play (Variables|Default|GetReloadStartSound) 0.0)
  (bind _outammo (Reload|AmmoUpdate (- (Variables|Configure|GetRoundMax) (Variables|Configure|GetRoundCurrent)) false))
  (bind _output_get (Variables|Configure|SetRoundCurrent _outammo))
  (if (!= _output_get 0)
    (Utilities|Time|SetTimerbyEvent (EventDispatchers|CreateEvent :!event AfterReloadDelayEnd) (Variables|Reload|GetCurrentReloadTime))
    (else
      (Variables|Default|SetWeaponState "NewEnumerator3")
      (Default|CallOnWeaponStatusChanged))))

(fn AmmoUpdate
  (params (InAmmo :type Integer) (Increased :type Boolean))
  (LocalVariables|SetL_Ammo InAmmo)
  (if Increased
    (if (> (Variables|Configure|GetAmmoCurrent) 0)
      _
      (elif (> (Variables|Configure|GetRoundCurrent) 0)
        _
        (else
          (Variables|Default|SetWeaponState "NewEnumerator1"))))
    (bind _output_get (LocalVariables|SetL_Current (+ (Variables|Configure|GetAmmoCurrent) (LocalVariables|GetL_Ammo))))
    (if (< _output_get (Variables|Configure|GetAmmoMax))
      (Variables|Configure|SetAmmoCurrent (LocalVariables|GetL_Current))
      (else
        (Variables|Configure|SetAmmoCurrent (Variables|Configure|GetAmmoMax))))
    (else
      (bind _output_get_2 (LocalVariables|SetL_Current (- (Variables|Configure|GetAmmoCurrent) (LocalVariables|GetL_Ammo))))
      (if (> _output_get_2 0)
        (Variables|Configure|SetAmmoCurrent (LocalVariables|GetL_Current))
        (else
          (Variables|Configure|SetAmmoCurrent 0)
          (Default|CallOnWeaponStatusChanged)
          (return (+ (Variables|Configure|GetRoundMax) (LocalVariables|GetL_Current)))))))
  (Default|CallOnWeaponStatusChanged)
  (return (Variables|Configure|GetRoundMax)))

(fn RoundsCount
  (bind _result (Math|Integer|DecrementInt (Variables|Configure|GetRoundCurrent))
    (:%20%20
      (return (> _result 0)))))

(fn AfterReloadDelayEnd
  (Variables|Default|SetWeaponState "NewEnumerator0")
  (Audio|Components|Audio|Play (Variables|Default|GetReloadEndSound) 0.0)
  (Default|CallOnWeaponStatusChanged))

(fn WeaponConfigure
  (params (InWeaponID :type Name))
  (Variables|Configure|SetWeaponID InWeaponID)
  (bind _returnvalue (Utilities|GetDataTableRow "/Game/DataTables/DT_Weapons.DT_Weapons" (Variables|Configure|GetWeaponID))
    (:then
      (Variables|Configure|SetWeaponStats _returnvalue)
      (Variables|Configure|SetCurrenWeaponType (.WeaponType (Utilities|Struct|BreakSTRUCT_WeaponStats (Variables|Configure|GetWeaponStats))))
      (Variables|Configure|SetRoundMax (.Rounds (Utilities|Struct|BreakSTRUCT_WeaponStats (Variables|Configure|GetWeaponStats))))
      (Variables|Configure|SetRoundCurrent (.Rounds (Utilities|Struct|BreakSTRUCT_WeaponStats (Variables|Configure|GetWeaponStats))))
      (Variables|Configure|SetCurrentDamage (.Damage (Utilities|Struct|BreakSTRUCT_WeaponStats (Variables|Configure|GetWeaponStats))))
      (Variables|Shoot|SetAfterShotDelay (.ShotTime (Utilities|Struct|BreakSTRUCT_WeaponStats (Variables|Configure|GetWeaponStats))))
      (Variables|Reload|SetCurrentReloadTime (.ReloadTime (Utilities|Struct|BreakSTRUCT_WeaponStats (Variables|Configure|GetWeaponStats))))
      (Variables|Reload|SetIsAutoReloading (.AutoReload (Utilities|Struct|BreakSTRUCT_WeaponStats (Variables|Configure|GetWeaponStats))))
      (Variables|Configure|SetCurrentRangeType (.RangeType (Utilities|Struct|BreakSTRUCT_WeaponStats (Variables|Configure|GetWeaponStats))))
      (Variables|Configure|SetCurrentRange (.Range (Utilities|Struct|BreakSTRUCT_WeaponStats (Variables|Configure|GetWeaponStats))))
      (Variables|Configure|SetAmmoMax (Utilities|Struct|BreakSTRUCT_WeaponStats (Variables|Configure|GetWeaponStats)))
      (Variables|Configure|SetAmmoCurrent (Variables|Configure|GetRoundMax))
      (if (Utilities|IsValid (Utilities|Struct|BreakSTRUCT_WeaponStats (Variables|Configure|GetWeaponStats)))
        (Components|StaticMesh|SetStaticMesh (Variables|Default|GetStaticMeshWeapon) (Utilities|Struct|BreakSTRUCT_WeaponStats (Variables|Configure|GetWeaponStats))))
      (bind _asbp_base_character (Utilities|Casting|CastToBP_BaseCharacter (Components|GetOwner))
        (:then
          (Variables|Configure|SetCurrentDamage (Math|Float|Truncate (* (Variables|Configure|GetCurrentDamage) (.DamageMult (Utilities|Struct|BreakSTRUCT_MainStats (Variables|/Game/Blueprints/Components/BP_MainStatsComp.BP_MainStatsComp_C|GetMainStats (Variables|/Game/Blueprints/Characters/BP_BaseCharacter.BP_BaseCharacter_C|GetBP_MainStatsComp _asbp_base_character)))))))
          (if (Utilities|IsValid (Variables|/Script/Engine.StaticMeshComponent|GetStaticMesh (Variables|Default|GetStaticMeshAim)))
            (Variables|Configure|SetIsAimExist true)
            (else
              (Rendering|Components|Light|SetIntensity (Variables|Default|GetPointLight) 0.0)
              (Rendering|Lighting|SetAttenuationRadius (Variables|Default|GetPointLight) 0.0)))
          (Variables|Configure|SetNickname (Utilities|Struct|BreakSTRUCT_WeaponStats (Variables|Configure|GetWeaponStats)))
          (return true))
        (:CastFailed
          (return false))))
    (:RowNotFound
      (return false))))

(fn AimUpdate
  (bind _aim (Variables|Default|GetAim))
  (bind _staticmeshaim (Variables|Default|GetStaticMeshAim))
  (bind _staticmeshaim_2 (Variables|Default|GetStaticMeshAim))
  (bind _returnvalue (Transformation|GetWorldScale _staticmeshaim))
  (bind _returnvalue_2 (Transformation|GetWorldScale _staticmeshaim_2))
  (bind _returnvalue_3 (Transformation|GetWorldLocation _aim))
  (if (Variables|Configure|GetIsAimExist)
    (bind (_outhit _returnvalue_4) (Collision|LineTraceByChannel _returnvalue_3 (+ _returnvalue_3 (* (Math|Vector|GetForwardVector _aim) 2e+03)) "TraceTypeQuery1" false 0 "None"))
    (if _returnvalue_4
      (LocalVariables|SetL_Dist (.Distance (Collision|BreakHitResult _outhit)))
      (LocalVariables|SetL_Loc (.Location (Collision|BreakHitResult _outhit)))
      (Transformation|SetWorldScale3D (Variables|Default|GetStaticMeshAim) (Math|Vector|MakeVector (/ (LocalVariables|GetL_Dist) 1e+03) (.y _returnvalue_2) (.z _returnvalue_2)))
      (Transformation|SetWorldLocation (Variables|Default|GetPointLight) (LocalVariables|GetL_Loc) false false)
      (Rendering|Components|Light|SetIntensity (Variables|Default|GetPointLight) 1e+03)
      (else
        (Transformation|SetWorldScale3D _staticmeshaim (Math|Vector|MakeVector 1.0 (.y _returnvalue) (.z _returnvalue)))
        (Transformation|SetWorldLocation (Variables|Default|GetPointLight) (Transformation|GetWorldLocation (Variables|Default|GetAim)) false false)
        (Rendering|Components|Light|SetIntensity (Variables|Default|GetPointLight) (Variables|Configure|GetAimLightIntencity))))))

(fn ActivateWeapon
  (params (Activation :type Boolean))
  (Variables|Configure|SetIsWeaponActive Activation)
  (LocalVariables|SetL_Skel (Actor|GetComponentsByClass "/Script/Engine.SkeletalMeshComponent"))
  (LocalVariables|SetL_Stat (Actor|GetComponentsByClass "/Script/Engine.StaticMeshComponent"))
  (Utilities|FlowControl|Sequence
    (:then_0
      (if (> (Utilities|Array|Length (LocalVariables|GetL_Skel)) 0)
        (for _array_element (LocalVariables|GetL_Skel)
          (Rendering|SetVisibility _array_element (Variables|Configure|GetIsWeaponActive) true))))
    (:then_1
      (if (> (Utilities|Array|Length (LocalVariables|GetL_Stat)) 0)
        (for _array_element_2 (LocalVariables|GetL_Stat)
          (Rendering|SetVisibility _array_element_2 (Variables|Configure|GetIsWeaponActive) true))))
    (:then_2
      (Rendering|Components|Light|SetIntensity (Variables|Default|GetPointLight) (Math|Float|SelectFloat (Variables|Configure|GetAimLightIntencity) 0.0 (Variables|Configure|GetIsWeaponActive))))
    (:then_3
      (if (Variables|Configure|GetIsWeaponActive)
        (Components|Activation|Activate (Variables|Default|GetPointLight) false)
        (else
          (Components|Activation|Deactivate (Variables|Default|GetPointLight)))))))