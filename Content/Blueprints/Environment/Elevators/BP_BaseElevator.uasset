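; BP_BaseElevator is a player-operated elevator that moves a platform between two fixed heights.
; Overlapping its Box with a BP_BaseCharacter enables input from player 0, and leaving disables it.
; The Use action flip-flops the ElevatorHights timeline between play and reverse.
; Timeline updates lerp the Plane's world Z between hard-coded absolute heights, keeping its X and Y.
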(event OnComponentBeginOverlap(Box)
  (params (OverlappedComponent :type Primitive%20Component%20Object%20Reference) (OtherActor :type Actor%20Object%20Reference) (OtherComp :type Primitive%20Component%20Object%20Reference) (OtherBodyIndex :type Integer) (bFromSweep :type Boolean) (SweepResult :type Hit%20Result%20Structure%20%28by%20ref%29))
  (Utilities|Casting|CastToBP_BaseCharacter OtherActor)
  (Input|EnableInput (Game|GetPlayerController 0)))

(event OnComponentEndOverlap(Box)
  (params (OverlappedComponent :type Primitive%20Component%20Object%20Reference) (OtherActor :type Actor%20Object%20Reference) (OtherComp :type Primitive%20Component%20Object%20Reference) (OtherBodyIndex :type Integer))
  (Utilities|Casting|CastToBP_BaseCharacter OtherActor)
  (Input|DisableInput (Game|GetPlayerController 0)))

(event Input|ActionEvents|InputActionUse
  (params (Key :type Key%20Structure :default "None"))
  (bind _plane (Variables|Default|GetPlane))
  (bind _returnvalue (Transformation|GetWorldLocation _plane))
  (:Pressed
    (Utilities|FlowControl|FlipFlop
      (:A
        (bind _z_value (Timeline|ElevatorHights Play)
          (:Update
            (Transformation|SetWorldLocation (Variables|Default|GetPlane) (Math|Vector|MakeVector (.x _returnvalue) (.y _returnvalue) (Math|Float|Lerp -5018.0 1.0 _z_value)) false false))))
      (:B
        (Timeline|ElevatorHights Reverse)))))

(fn ConstructionScript)