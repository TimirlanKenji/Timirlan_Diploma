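; BP_CustomSpawner is a spawner actor that creates a set number of NPCs at its spawn point, one at a time.
; It can begin on BeginPlay or through StartSpawnNPCs, and a delay timer paces the spawns until the count is reached or StopSpawnNPCs is called.
; When a patrolling group is set, each new BP_BaseNPC receives that group and its BP_CustomAIController's AI state is switched for patrolling.
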(event EventBeginPlay
  (|CallParentFunction)
  (if (Variables|Default|GetSpawnOnStart)
    (CallFunction|StartSpawnNPCs)))

(event Collision|EventActorBeginOverlap
  (params (OtherActor :type Actor%20Object%20Reference))
  (|CallParentFunction OtherActor) ; This node is disabled and will not be called.\nDrag off pins to build functionality.
)

(event EventTick
  (params (DeltaSeconds :type Float%20%28single-precision%29))
  (|CallParentFunction DeltaSeconds) ; This node is disabled and will not be called.\nDrag off pins to build functionality.
)

(fn ConstructionScript
  (|CallParentFunction))

(fn SpawnOneNPC
  (if (not (Variables|Default|GetIsDone))
    (if (Utilities|IsValidClass (Variables|Default|GetSpawnNPCClass))
      (if (< (Variables|Default|GetCounter) (Variables|Default|GetNPCsCont))
        (bind _returnvalue (Game|SpawnActorfromClass (Variables|Default|GetSpawnNPCClass) (Transformation|GetWorldTransform (Variables|Default|GetSpawnPoint)) "AdjustIfPossibleButAlwaysSpawn" 0 0))
        (bind _asbp_base_npc (Utilities|Casting|CastToBP_BaseNPC _returnvalue))
        (Variables|Default|SetLastSpawnedNPC _asbp_base_npc)
        (CallFunction|UpdatePatrolStateforSpawnedNPC)
        (Math|Integer|IncrementInt (Variables|Default|GetCounter)
          (:%20%20
            (Utilities|Time|SetTimerbyEvent (EventDispatchers|CreateEvent :!event SpawnOneNPC) (Variables|Default|GetBetweenSpawnDelay))))
        (else
          (Variables|Default|SetIsDone true))))))

(fn StartSpawnNPCs
  (CallFunction|SpawnOneNPC))

(fn StopSpawnNPCs
  (Variables|Default|SetIsDone true))

(fn UpdatePatrolStateforSpawnedNPC
  (if (!= (Variables|Default|GetPatrollingGroup) 0)
    (Variables|/Game/Blueprints/Characters/NPC/BP_BaseNPC.BP_BaseNPC_C|SetPatrollingGroup (Variables|Default|GetLastSpawnedNPC) (Variables|Default|GetPatrollingGroup))
    (bind _asbp_custom_aicontroller (Utilities|Casting|CastToBP_CustomAIController (AI|GetAIController (Variables|Default|GetLastSpawnedNPC))))
    (Variables|/Game/Blueprints/Controllers/BP_CustomAIController.BP_CustomAIController_C|SetAIState _asbp_custom_aicontroller "NewEnumerator1")))