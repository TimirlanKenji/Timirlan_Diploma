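; BP_RestoringItem is a spinning pickup that restores health and shield to actors with a BP_MainStatsComp.
; Tick yaws the mesh, while overlapping the collision sphere calls HealUp and ShieldUp for each positive value whose stat is not already maxed.
; Both calls share the HealUpToMaximum flag, so shield has no separate fill-to-max setting.
; The item destroys itself only if it restored something, otherwise it stays in the world.
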(event OnComponentBeginOverlap(SphereCollision)
  (params (OverlappedComponent :type Primitive%20Component%20Object%20Reference) (OtherActor :type Actor%20Object%20Reference) (OtherComp :type Primitive%20Component%20Object%20Reference) (OtherBodyIndex :type Integer) (bFromSweep :type Boolean) (SweepResult :type Hit%20Result%20Structure%20%28by%20ref%29))
  (bind _returnvalue (Actor|GetComponentbyClass OtherActor "/Game/Blueprints/Components/BP_MainStatsComp.BP_MainStatsComp_C"))
  ;[1 1 1] Main Stats Comp check
  (Utilities|IsValid _returnvalue
    (:Is%20Valid
      (Variables|Default|SetCurrentMainStats _returnvalue)
      (Utilities|FlowControl|Sequence
        (:then_0
          (if (> (Variables|Default|GetHealUpValue) 0)
            ;[1 1 1] Check HP on Max
            (if (not (Default|CheckHP (Variables|Default|GetCurrentMainStats)))
              ;[1 1 1] MainStatsComp HealUp
              (Default|HealUp (Variables|Default|GetCurrentMainStats) (Variables|Default|GetHealUpToMaximum) (Variables|Default|GetHealUpValue))
              (Variables|Default|SetIsItUseful true))))
        (:then_1
          (if (> (Variables|Default|GetShieldUpValue) 0)
            ;[1 1 1] Check EP on Max
            (if (not (Default|CheckEP (Variables|Default|GetCurrentMainStats)))
              ;[1 1 1] MainStatsComp ShieldUp
              (Default|ShieldUp (Variables|Default|GetCurrentMainStats) (Variables|Default|GetHealUpToMaximum) (Variables|Default|GetShieldUpValue))
              (Variables|Default|SetIsItUseful true))))
        (:then_2
          (if (Variables|Default|GetIsItUseful)
            (Actor|DestroyActor)))))))

(event EventBeginPlay
  (|CallParentFunction) ; This node is disabled and will not be called.\nDrag off pins to build functionality.
)

(event Collision|EventActorBeginOverlap
  (params (OtherActor :type Actor%20Object%20Reference))
  (|CallParentFunction OtherActor) ; This node is disabled and will not be called.\nDrag off pins to build functionality.
)

(event EventTick
  (params (DeltaSeconds :type Float%20%28single-precision%29))
  (|CallParentFunction DeltaSeconds)
  (Transformation|AddRelativeRotation (Variables|Default|GetStaticMesh) (Math|Rotator|MakeRotator 0.0 0.0 (Variables|Default|GetRotationSpeed)) false false))

(fn ConstructionScript
  (|CallParentFunction))