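; BP_AmmoToPick is an ammo pickup that spins from a random starting yaw.
; When a BP_PlayerCharacter enters its sphere collision, it looks up the weapon matching its ammo type ID in the player's weapon map and increases that weapon's ammo.
; The pickup destroys itself only if a matching weapon was found, otherwise it stays in the world.
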(event OnComponentBeginOverlap(SphereCollision)
  (params (OverlappedComponent :type Primitive%20Component%20Object%20Reference) (OtherActor :type Actor%20Object%20Reference) (OtherComp :type Primitive%20Component%20Object%20Reference) (OtherBodyIndex :type Integer) (bFromSweep :type Boolean) (SweepResult :type Hit%20Result%20Structure%20%28by%20ref%29))
  ;[1 1 1] Main Stats Comp check
  (bind _asbp_player_character (Utilities|Casting|CastToBP_PlayerCharacter OtherActor))
  (Variables|Default|SetPlayerCharacter _asbp_player_character)
  (Utilities|FlowControl|Sequence
    (:then_0
      (CallFunction|AddAmmotoWeapon))
    (:then_1
      (if (Variables|Default|GetIsItUseful)
        (Actor|DestroyActor)))))

(event EventBeginPlay
  (|CallParentFunction)
  (Transformation|AddRelativeRotation (Variables|Default|GetStaticMesh) (Math|Rotator|MakeRotator 0.0 0.0 (Math|Random|RandomFloatinRange 0.0 3.6e+02)) false false))

(event Collision|EventActorBeginOverlap
  (params (OtherActor :type Actor%20Object%20Reference))
  (|CallParentFunction OtherActor) ; This node is disabled and will not be called.\nDrag off pins to build functionality.
)

(event EventTick
  (params (DeltaSeconds :type Float%20%28single-precision%29))
  (|CallParentFunction DeltaSeconds)
  (Transformation|AddRelativeRotation (Variables|Default|GetStaticMesh) (Math|Rotator|MakeRotator 0.0 0.0 (Variables|Default|GetRotationSpeed)) false false))

(fn ConstructionScript
  (|CallParentFunction))

(fn AddAmmotoWeapon
  (bind _playercharacter (Variables|Default|GetPlayerCharacter))
  (bind _ammotypebyid (Variables|Default|GetAmmoTypeByID))
  (bind _mapofweapon (Variables|/Game/Blueprints/Characters/BP_BaseCharacter.BP_BaseCharacter_C|GetMapOfWeapon _playercharacter))
  (bind (_value _returnvalue) (Utilities|Map|Find _mapofweapon _ammotypebyid))
  (if (Utilities|Name|NotEqual(Name) (Variables|Default|GetAmmoTypeByID) "None")
    (if _returnvalue
      (LocalVariables|SetL_Weap _value)
      (Default|AmmoUpdate (LocalVariables|GetL_Weap) (Variables|Default|GetAmmoToAdd) true)
      (Variables|Default|SetIsItUseful true))))