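; Customizable trap trigger actor whose Construction Script builds a row of repeated meshes along local X from the Count and Space variables.
; One loop copies StaticMesh's mesh at unit scale, and a second copies StaticMesh1's mesh at its world scale, also adding an unconfigured material billboard per step.
; BeginPlay applies a red material to the two source components only.
; The graph contains no active overlap or trap logic of its own.
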(event EventBeginPlay
  (|CallParentFunction)
  (Rendering|Material|SetMaterial (Variables|Default|GetStaticMesh) 0 "/Game/Blueprints/Components/Art/Shaders/MI_BaseColor_Red.MI_BaseColor_Red")
  (Rendering|Material|SetMaterial (Variables|Default|GetStaticMesh1) 0 "/Game/Blueprints/Components/Art/Shaders/MI_BaseColor_Red.MI_BaseColor_Red"))

(event Collision|EventActorBeginOverlap
  (params (OtherActor :type Actor%20Object%20Reference))
  (|CallParentFunction OtherActor) ; This node is disabled and will not be called.\nDrag off pins to build functionality.
)

(event EventTick
  (params (DeltaSeconds :type Float%20%28single-precision%29))
  (|CallParentFunction DeltaSeconds) ; This node is disabled and will not be called.\nDrag off pins to build functionality.
)

(fn ConstructionScript
  (|CallParentFunction)
  (Utilities|FlowControl|Sequence
    (:then_0
      (for _index (range 0 (Variables|Default|GetCount))
        (bind _returnvalue (AddComponent|AddStaticMeshComponent false (Math|Transform|MakeTransform (Math|Vector|MakeVector (Math|Conversions|ToFloat(Integer) (* _index (Variables|Default|GetSpace))) 0.0 0.0))))
        (Components|StaticMesh|SetStaticMesh _returnvalue (Variables|/Script/Engine.StaticMeshComponent|GetStaticMesh (Variables|Default|GetStaticMesh)))))
    (:then_1
      (for _index_2 (range 0 (Variables|Default|GetCount))
        (bind _returnvalue_2 (AddComponent|AddStaticMeshComponent false (Math|Transform|MakeTransform (Math|Vector|MakeVector (Math|Conversions|ToFloat(Integer) (* _index_2 (Variables|Default|GetSpace))) 0.0 0.0) "0, 0, 0" (Transformation|GetWorldScale (Variables|Default|GetStaticMesh1)))))
        (Components|StaticMesh|SetStaticMesh _returnvalue_2 (Variables|/Script/Engine.StaticMeshComponent|GetStaticMesh (Variables|Default|GetStaticMesh1)))
        (AddComponent|AddMaterialBillboardComponent (Components|GetOwner (Variables|Default|GetStaticMesh)) false)))))