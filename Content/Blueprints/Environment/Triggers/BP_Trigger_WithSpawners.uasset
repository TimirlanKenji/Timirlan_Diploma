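; A trigger actor that starts NPC spawning on a set of linked spawners when the player character enters its box.
; On overlap it registers itself as the player's custom actor and calls start on every spawner in its list.
; On exit, only if the stop-on-end-overlap flag is set, it clears that reference and stops the spawners.
; Its Interact override simply returns the parent's result.
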(event OnComponentBeginOverlap(Box)
  (params (OverlappedComponent :type Primitive%20Component%20Object%20Reference) (OtherActor :type Actor%20Object%20Reference) (OtherComp :type Primitive%20Component%20Object%20Reference) (OtherBodyIndex :type Integer) (bFromSweep :type Boolean) (SweepResult :type Hit%20Result%20Structure%20%28by%20ref%29))
  (bind _asbp_player_character (Utilities|Casting|CastToBP_PlayerCharacter OtherActor))
  (Default|UpdateCustomActor _asbp_player_character self)
  (for _array_element (Variables|Default|GetSpawnersToInteract)
    (Default|StartSpawnNPCs _array_element)))

(event OnComponentEndOverlap(Box)
  (params (OverlappedComponent :type Primitive%20Component%20Object%20Reference) (OtherActor :type Actor%20Object%20Reference) (OtherComp :type Primitive%20Component%20Object%20Reference) (OtherBodyIndex :type Integer))
  (bind _asbp_player_character (Utilities|Casting|CastToBP_PlayerCharacter OtherActor))
  (if (Variables|Default|GetStopSpawningOnEndOverlap)
    (Default|UpdateCustomActor _asbp_player_character)
    (for _array_element (Variables|Default|GetSpawnersToInteract)
      (Default|StopSpawnNPCs _array_element))))

(event EventBeginPlay
  (|CallParentFunction) ; This node is disabled and will not be called.\nDrag off pins to build functionality.
)

(event Collision|EventActorBeginOverlap
  (params (OtherActor :type Actor%20Object%20Reference))
  (|CallParentFunction OtherActor) ; This node is disabled and will not be called.\nDrag off pins to build functionality.
)

(event EventTick
  (params (DeltaSeconds :type Float%20%28single-precision%29))
  (|CallParentFunction DeltaSeconds) ; This node is disabled and will not be called.\nDrag off pins to build functionality.
)

(fn ConstructionScript
  (|CallParentFunction))

(fn Interact
  (bind _success (|CallParentFunction))
  (bind _output_get (LocalVariables|SetL_Success _success))
  (return _output_get))