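; BP_Trigger_WithDoors2 is an interactable box trigger that controls the doors listed in DoorToInteract.
; When a BP_BaseCharacter enters the box, it registers itself as that character's custom actor and opens the doors; on exit it clears that reference and closes them.
; Its Interact override calls the parent, toggles the lock on linked BP_DoorWithLock doors through SwitchDoorsLocks, and always returns true.
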(event OnComponentBeginOverlap(Box)
  (params (OverlappedComponent :type Primitive%20Component%20Object%20Reference) (OtherActor :type Actor%20Object%20Reference) (OtherComp :type Primitive%20Component%20Object%20Reference) (OtherBodyIndex :type Integer) (bFromSweep :type Boolean) (SweepResult :type Hit%20Result%20Structure%20%28by%20ref%29))
  (bind _asbp_base_character (Utilities|Casting|CastToBP_BaseCharacter OtherActor))
  (Default|UpdateCustomActor _asbp_base_character self)
  (for _array_element (Variables|Default|GetDoorToInteract)
    (Default|DoorOpen _array_element)))

(event OnComponentEndOverlap(Box)
  (params (OverlappedComponent :type Primitive%20Component%20Object%20Reference) (OtherActor :type Actor%20Object%20Reference) (OtherComp :type Primitive%20Component%20Object%20Reference) (OtherBodyIndex :type Integer))
  (bind _asbp_base_character (Utilities|Casting|CastToBP_BaseCharacter OtherActor))
  (Default|UpdateCustomActor _asbp_base_character)
  (for _array_element (Variables|Default|GetDoorToInteract)
    (Default|DoorClose _array_element)))

(event EventBeginPlay
  (|CallParentFunction) ; This node is disabled and will not be called.\nDrag off pins to build functionality.
)

(event Collision|EventActorBeginOverlap
  (params (OtherActor :type Actor%20Object%20Reference))
  (|CallParentFunction OtherActor) ; This node is disabled and will not be called.\nDrag off pins to build functionality.
)

(event EventTick
  (params (DeltaSeconds :type Float%20%28single-precision%29))
  (|CallParentFunction DeltaSeconds) ; This node is disabled and will not be called.\nDrag off pins to build functionality.
)

(fn ConstructionScript
  (|CallParentFunction))

(fn Interact
  (bind _success (|CallParentFunction))
  (LocalVariables|SetL_Success _success)
  (CallFunction|SwitchDoorsLocks)
  (return true))

(fn SwitchDoorsLocks
  (for _array_element (Variables|Default|GetDoorToInteract)
    (bind _asbp_door_with_lock (Utilities|Casting|CastToBP_DoorWithLock _array_element))
    (Default|SwitchLock _asbp_door_with_lock)))