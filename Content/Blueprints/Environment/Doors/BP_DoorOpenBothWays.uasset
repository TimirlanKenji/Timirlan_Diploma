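; Door Blueprint, named for opening both ways, that sets up an optionally pre-opened door with a configurable overlap box.
; The construction script yaws SceneDoor by the maximum open angle when IsOpen is set, then sizes Box1 and raises it by its Z extent.
; BeginPlay calls the parent and applies EnableOverlap to the box; this graph contains no swing or overlap-response logic.
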(event EventBeginPlay
  (|CallParentFunction)
  (Variables|/Script/Engine.PrimitiveComponent|SetbGenerateOverlapEvents (Variables|Default|GetBox1) (Variables|Default|GetEnableOverlap)))

(event Collision|EventActorBeginOverlap
  (params (OtherActor :type Actor%20Object%20Reference))
  (|CallParentFunction OtherActor) ; This node is disabled and will not be called.\nDrag off pins to build functionality.
)

(event EventTick
  (params (DeltaSeconds :type Float%20%28single-precision%29))
  (|CallParentFunction DeltaSeconds) ; This node is disabled and will not be called.\nDrag off pins to build functionality.
)

(fn ConstructionScript
  (|CallParentFunction)
  (Utilities|FlowControl|Sequence
    (:then_0
      (Transformation|AddRelativeRotation (Variables|Default|GetSceneDoor) (Math|Rotator|MakeRotator 0.0 0.0 (select (Variables|Default|GetIsOpen) (Variables|Default|GetMaxDoorOpenAngle) 0.0)) false false))
    (:then_1
      (Components|Box|SetBoxExtent (Variables|Default|GetBox1) (Variables|Default|GetExtent) true)
      (Transformation|AddRelativeLocation (Variables|Default|GetBox1) (Math|Vector|MakeVector 0.0 0.0 (.Z (Math|Vector|BreakVector (Variables|Default|GetExtent)))) false false))))