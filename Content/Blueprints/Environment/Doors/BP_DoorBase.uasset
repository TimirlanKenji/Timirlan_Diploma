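; BP_DoorBase is a base door that swings open when a BP_BaseCharacter enters its box trigger and closes when the character leaves.
; One timeline, played forward or in reverse, drives the door's yaw up to MaxDoorOpenAngle, ignoring new requests while moving.
; Overlaps also set or clear the door as the character's custom actor.
; Construction applies the initial open state and sizes and raises the trigger; BeginPlay toggles its overlap events.
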(event OnComponentBeginOverlap(Box)
  (params (OverlappedComponent :type Primitive%20Component%20Object%20Reference) (OtherActor :type Actor%20Object%20Reference) (OtherComp :type Primitive%20Component%20Object%20Reference) (OtherBodyIndex :type Integer) (bFromSweep :type Boolean) (SweepResult :type Hit%20Result%20Structure%20%28by%20ref%29))
  (bind _asbp_base_character (Utilities|Casting|CastToBP_BaseCharacter OtherActor))
  (CallFunction|DoorOpen)
  (Default|UpdateCustomActor _asbp_base_character self))

(event OnComponentEndOverlap(Box)
  (params (OverlappedComponent :type Primitive%20Component%20Object%20Reference) (OtherActor :type Actor%20Object%20Reference) (OtherComp :type Primitive%20Component%20Object%20Reference) (OtherBodyIndex :type Integer))
  (bind _asbp_base_character (Utilities|Casting|CastToBP_BaseCharacter OtherActor))
  (CallFunction|DoorClose)
  (Default|UpdateCustomActor _asbp_base_character))

(event Custom|DoorOpen
  (if (not (Variables|Default|GetInProgress))
    (if (not (Variables|DoorConfigure|GetIsOpen))
      (bind (_direction _openprogression) (Timeline|Timeline_0 PlayFromStart)
        (:Update
          (Variables|Default|SetInProgress true)
          (Transformation|SetRelativeRotation (Variables|Default|GetSceneDoor) (Math|Rotator|MakeRotator 0.0 0.0 (* (Variables|DoorConfigure|GetMaxDoorOpenAngle) _openprogression)) false false))
        (:Finished
          (Variables|Default|SetInProgress false)
          (switch Utilities|FlowControl|Switch|SwitchonETimelineDirection _direction
            (:Forward
              (Variables|DoorConfigure|SetIsOpen true))
            (:Backward
              (Variables|DoorConfigure|SetIsOpen false))))))))

(event Custom|DoorClose
  (if (not (Variables|Default|GetInProgress))
    (if (Variables|DoorConfigure|GetIsOpen)
      (bind (_direction _openprogression) (Timeline|Timeline_0 ReverseFromEnd)
        (:Update
          (Variables|Default|SetInProgress true)
          (Transformation|SetRelativeRotation (Variables|Default|GetSceneDoor) (Math|Rotator|MakeRotator 0.0 0.0 (* (Variables|DoorConfigure|GetMaxDoorOpenAngle) _openprogression)) false false))
        (:Finished
          (Variables|Default|SetInProgress false)
          (switch Utilities|FlowControl|Switch|SwitchonETimelineDirection _direction
            (:Forward
              (Variables|DoorConfigure|SetIsOpen true))
            (:Backward
              (Variables|DoorConfigure|SetIsOpen false))))))))

(event EventBeginPlay
  (Variables|/Script/Engine.PrimitiveComponent|SetbGenerateOverlapEvents (Variables|Default|GetBox) (Variables|DoorConfigure|GetEnableOverlap)))

(event EventTick
  (params (DeltaSeconds :type Float%20%28single-precision%29)))

(fn ConstructionScript
  (Utilities|FlowControl|Sequence
    (:then_0
      (Transformation|AddRelativeRotation (Variables|Default|GetSceneDoor) (Math|Rotator|MakeRotator 0.0 0.0 (select (Variables|DoorConfigure|GetIsOpen) (Variables|DoorConfigure|GetMaxDoorOpenAngle) 0.0)) false false))
    (:then_1
      (Components|Box|SetBoxExtent (Variables|Default|GetBox) (Variables|DoorConfigure|GetExtent) true)
      (Transformation|AddRelativeLocation (Variables|Default|GetBox) (Math|Vector|MakeVector 0.0 0.0 (.Z (Math|Vector|BreakVector (Variables|DoorConfigure|GetExtent)))) false false))))