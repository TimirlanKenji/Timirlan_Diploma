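; BP_DoorWithLock is a child door Blueprint that adds a lock, blocking opening and closing while locked.
; DoorOpen and DoorClose call the parent logic only when IsLocked is false.
; Interact runs the parent interaction, then toggles the lock through SwitchLock and always returns true.
; A point light shows the state, dark red and brighter when locked or green when unlocked, set at construction and on each toggle.
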(event EventBeginPlay
  (|CallParentFunction) ; This node is disabled and will not be called.\nDrag off pins to build functionality.
)

(event Collision|EventActorBeginOverlap
  (params (OtherActor :type Actor%20Object%20Reference))
  (|CallParentFunction OtherActor) ; This node is disabled and will not be called.\nDrag off pins to build functionality.
)

(event EventTick
  (params (DeltaSeconds :type Float%20%28single-precision%29))
  (|CallParentFunction DeltaSeconds) ; This node is disabled and will not be called.\nDrag off pins to build functionality.
)

(event EventDoorOpen
  (if (not (Variables|Default|GetIsLocked))
    (|CallParentFunction)))

(event EventDoorClose
  (if (not (Variables|Default|GetIsLocked))
    (|CallParentFunction)))

(fn ConstructionScript
  (|CallParentFunction)
  (CallFunction|SetLightProperities))

(fn SwitchLock
  (Variables|Default|SetIsLocked (not (Variables|Default|GetIsLocked)))
  (CallFunction|SetLightProperities))

(fn SetLightProperities
  (Rendering|Components|Light|SetIntensity (Variables|Default|GetPointLight) (select (Variables|Default|GetIsLocked) 5e+03 3e+03))
  (Rendering|Components|Light|SetLightColor (Variables|Default|GetPointLight) (select (Variables|Default|GetIsLocked) "(R=0.307292,G=0.019206,B=0.062738,A=1.000000)" "(R=0.184528,G=0.666667,B=0.000000,A=1.000000)") true))

(fn TestFunc
  (|CallParentFunction))

(fn Interact
  (bind _success (|CallParentFunction))
  (LocalVariables|SetL_Success _success)
  (CallFunction|SwitchLock)
  (return true))