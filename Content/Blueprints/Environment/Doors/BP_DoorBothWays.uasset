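; BP_DoorBothWays is a door actor that toggles open and closed with the Use input action.
; A BP_BaseCharacter overlapping Box100 enables input for player 0 on the door, and leaving disables it.
; Use drives a FlipFlop that alternately plays and reverses a timeline, whose updates add a lerped yaw delta to SceneDoorOpen rather than setting an absolute rotation.
; Despite the name, no side-dependent direction logic is connected.
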(event OnComponentBeginOverlap(Box100)
  (params (OverlappedComponent :type Primitive%20Component%20Object%20Reference) (OtherActor :type Actor%20Object%20Reference) (OtherComp :type Primitive%20Component%20Object%20Reference) (OtherBodyIndex :type Integer) (bFromSweep :type Boolean) (SweepResult :type Hit%20Result%20Structure%20%28by%20ref%29))
  ;[1 1 1] Enable input
  (Utilities|Casting|CastToBP_BaseCharacter OtherActor)
  (Input|EnableInput (Game|GetPlayerController 0)))

(event OnComponentEndOverlap(Box100)
  (params (OverlappedComponent :type Primitive%20Component%20Object%20Reference) (OtherActor :type Actor%20Object%20Reference) (OtherComp :type Primitive%20Component%20Object%20Reference) (OtherBodyIndex :type Integer))
  ;[1 1 1] Disable input
  (Utilities|Casting|CastToBP_BaseCharacter OtherActor)
  (Input|DisableInput (Game|GetPlayerController 0)))

(event Input|ActionEvents|InputActionUse
  (params (Key :type Key%20Structure :default "None"))
  (:Pressed
    (Utilities|FlowControl|FlipFlop
      (:A
        (bind _z_value (Timeline|Timeline_0 Play)
          (:Update
            (Transformation|AddRelativeRotation (Variables|Default|GetSceneDoorOpen) (Math|Rotator|MakeRotator 0.0 0.0 (Math|Float|Lerp 1e+02 -1e+02 _z_value)) false false))))
      (:B
        (Timeline|Timeline_0 Reverse)))))

(fn ConstructionScript)