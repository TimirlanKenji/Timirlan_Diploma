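; Base spline actor that builds meshes along an editable spline in the construction script, with optional closed loop and collision.
; It syncs a per-point toggle array to the point count, then adds a spline mesh per segment and an optional static mesh at flagged points.
; It also places start and end meshes and can label points with numbered text.
; GenerateMainSplineMesh is marked obsolete and unused.
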(fn ConstructionScript
  (Utilities|FlowControl|Sequence
    (:then_0
      (CallFunction|UpdateSplinePointsCount)
      (CallFunction|BuildSplineDataArray))
    (:then_1
      (CallFunction|MakeLoop))
    (:then_2
      (CallFunction|GenerateStartMesh)
      (CallFunction|GenerateEndMesh)
      (CallFunction|SplinePointsNumbers))))

(fn GenerateMainSplineMesh
  ;[0 0 0] OBSOLETE
  (for _index (range 0 (Variables|Default|GetSplinePointsCount))
    (LocalVariables|SetL_Index _index)
    (if (< (LocalVariables|GetL_Index) (- (Variables|Default|GetSplinePointsCount) 1))
      (bind _returnvalue (AddComponent|AddSplineMeshComponent false))
      (bind _output_get (LocalVariables|SetL_MainSplineMeshComp _returnvalue))
      (Collision|SetCollisionEnabled _output_get (select (Variables|Tools|GetIsCollisionEnabled) "QueryOnly" "NoCollision"))
      (Components|StaticMesh|SetStaticMesh (LocalVariables|GetL_MainSplineMeshComp) (Variables|Meshes|GetMainSplineMesh))
      (SplineMesh|SetStartandEnd (LocalVariables|GetL_MainSplineMeshComp) (.Location (Spline|GetLocationandTangentatSplinePoint (Variables|Default|GetSpline) (LocalVariables|GetL_Index) "Local")) (.Tangent (Spline|GetLocationandTangentatSplinePoint (Variables|Default|GetSpline) (LocalVariables|GetL_Index) "Local")) (.Location (Spline|GetLocationandTangentatSplinePoint (Variables|Default|GetSpline) (+ (LocalVariables|GetL_Index) 1) "Local")) (.Tangent (Spline|GetLocationandTangentatSplinePoint (Variables|Default|GetSpline) (+ (LocalVariables|GetL_Index) 1) "Local")) true :!class /Script/Engine.SplineMeshComponent))))

(fn GenerateStartMesh
  (CallFunction|GenerateMeshonPoint (Variables|Meshes|GetStartMesh)))

(fn GenerateEndMesh
  (CallFunction|GenerateMeshonPoint (Variables|Meshes|GetEndMesh) (select (Variables|Points|GetIsItInLoop) 0 (Variables|Default|GetSplinePointsCount))))

(fn GenerateMeshonPoint
  (params (InStaticMesh :type Static%20Mesh%20Object%20Reference) (InPoint :type Integer))
  (bind _output_get (LocalVariables|SetL_StaticMeshObj InStaticMesh))
  (Utilities|IsValid _output_get
    (:Is%20Valid
      (LocalVariables|SetL_PointIndex InPoint)
      (if (> (Variables|Default|GetSplinePointsCount) 0)
        (bind _returnvalue (AddComponent|AddStaticMeshComponent false (Spline|GetTransformatSplinePoint (Variables|Default|GetSpline) (LocalVariables|GetL_PointIndex) "Local" false)))
        (Components|StaticMesh|SetStaticMesh _returnvalue (LocalVariables|GetL_StaticMeshObj))))))

(fn GenerateMeshonEachPoint)

(fn UpdateSplinePointsCount
  (Variables|Default|SetSplinePointsCount (Spline|GetNumberOfSplinePoints (Variables|Default|GetSpline))))

(fn BuildSplineDataArray
  (Math|Integer|CompareInt (Utilities|Array|Length (Variables|Points|GetMeshInPoint)) (Variables|Default|GetSplinePointsCount) :!label _label
    (:>
      (Utilities|Array|RemoveIndex (Variables|Points|GetMeshInPoint) (Utilities|Array|LastIndex (Variables|Points|GetMeshInPoint)))
      (goto _label))
    (:<
      (Utilities|Array|Add (Variables|Points|GetMeshInPoint) (Variables|Points|GetMeshInPointDefault))
      (goto _label))))

(fn MakeLoop
  (for _index (range 0 (- (Variables|Default|GetSplinePointsCount) (Math|Integer|SelectInt 1 2 (Variables|Points|GetIsItInLoop))))
    (bind _output_get (Variables|Default|SetCurrentLoopIndex _index))
    (CallFunction|BuildSplineMeshElement _output_get (Variables|Meshes|GetMainSplineMesh))
    (if (Utilities|Array|Get(acopy) (Variables|Points|GetMeshInPoint) (Variables|Default|GetCurrentLoopIndex))
      (CallFunction|GenerateMeshonPoint (Variables|Meshes|GetOnPointMesh) (Variables|Default|GetCurrentLoopIndex))))
  (if (Utilities|Array|Get(acopy) (Variables|Points|GetMeshInPoint) (+ (Variables|Default|GetCurrentLoopIndex) 1))
    (CallFunction|GenerateMeshonPoint (Variables|Meshes|GetOnPointMesh) (+ (Variables|Default|GetCurrentLoopIndex) 1))))

(fn BuildSplineMeshElement
  (params (InLoopIndex :type Integer) (InStaticMesh :type Static%20Mesh%20Object%20Reference))
  (bind _returnvalue (+ InLoopIndex 1))
  (LocalVariables|SetL_CurrentLoopIndex InLoopIndex)
  (LocalVariables|SetL_NextLoopIndex (select (Variables|Points|GetIsItInLoop) (Math|Integer|%(Integer) _returnvalue (Variables|Default|GetSplinePointsCount)) _returnvalue))
  (LocalVariables|SetL_SplineElementMesh InStaticMesh)
  (Utilities|FlowControl|Sequence
    (:then_0
      (LocalVariables|SetL_StartLocation (.Location (Spline|GetLocationandTangentatSplinePoint (Variables|Default|GetSpline) (LocalVariables|GetL_CurrentLoopIndex) "Local")))
      (LocalVariables|SetL_StartTangent (.Tangent (Spline|GetLocationandTangentatSplinePoint (Variables|Default|GetSpline) (LocalVariables|GetL_CurrentLoopIndex) "Local")))
      (LocalVariables|SetL_EndLocation (.Location (Spline|GetLocationandTangentatSplinePoint (Variables|Default|GetSpline) (LocalVariables|GetL_NextLoopIndex) "Local")))
      (LocalVariables|SetL_EndTangent (.Tangent (Spline|GetLocationandTangentatSplinePoint (Variables|Default|GetSpline) (LocalVariables|GetL_NextLoopIndex) "Local"))))
    (:then_1
      (bind _returnvalue_2 (AddComponent|AddSplineMeshComponent false))
      (bind _output_get (LocalVariables|SetL_CurrentSplineMesh _returnvalue_2))
      (Components|StaticMesh|SetStaticMesh _output_get (LocalVariables|GetL_SplineElementMesh))
      (SplineMesh|SetStartandEnd (LocalVariables|GetL_CurrentSplineMesh) (LocalVariables|GetL_StartLocation) (LocalVariables|GetL_StartTangent) (LocalVariables|GetL_EndLocation) (LocalVariables|GetL_EndTangent) true :!class /Script/Engine.SplineMeshComponent)
      (Collision|SetCollisionEnabled (LocalVariables|GetL_CurrentSplineMesh) (select (Variables|Tools|GetIsCollisionEnabled) "QueryOnly" "NoCollision")))))

(fn SplinePointsNumbers
  (if (Variables|Tools|GetIsSplinepointsNumbersEnabled)
    (for _index (range 0 (- (Variables|Default|GetSplinePointsCount) 1))
      (LocalVariables|SetL_CurrentPoint (Utilities|Text|ToText(Integer) _index))
      (bind _returnvalue (AddComponent|AddTextRenderComponent false (Math|Transform|MakeTransform (Math|Vector|MakeVector (.X (Math|Vector|BreakVector (.Location (Spline|GetLocationandTangentatSplinePoint (Variables|Default|GetSpline) _index "Local")))) (.Y (Math|Vector|BreakVector (.Location (Spline|GetLocationandTangentatSplinePoint (Variables|Default|GetSpline) _index "Local")))) (+ (.Z (Math|Vector|BreakVector (.Location (Spline|GetLocationandTangentatSplinePoint (Variables|Default|GetSpline) _index "Local")))) (Math|Conversions|ToFloat(Integer) (Variables|Tools|GetZPosition)))) (Math|Conversions|RotationFromXVector (* (.Tangent (Spline|GetLocationandTangentatSplinePoint (Variables|Default|GetSpline) _index "Local")) -1.0)))))
      (Rendering|Components|TextRender|SetText _returnvalue (LocalVariables|GetL_CurrentPoint)))))