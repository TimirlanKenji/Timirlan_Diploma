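; HUD Blueprint for the menu that shows the main menu widget as soon as play begins.
; BeginPlay flags the menu as open, sets the widget type to an enum value, calls UpdateMainMenuWidget and adds WidgetMainMenu to the viewport.
; It then switches the first player controller to UI-only input, focused on that widget with the mouse unlocked.
; UpdateMainMenuWidget is not defined in this graph.
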(event EventBeginPlay
  (Variables|Default|SetIsMenuOpen true)
  (Variables|Default|SetIsWidgetType "NewEnumerator0")
  (CallFunction|UpdateMainMenuWidget)
  (UserInterface|Viewport|AddtoViewport (Variables|Default|GetWidgetMainMenu) 0)
  (Input|SetInputModeUIOnly (Game|GetPlayerController 0) (Variables|Default|GetWidgetMainMenu) "DoNotLock"))

(event Collision|EventActorBeginOverlap
  (params (OtherActor :type Actor%20Object%20Reference))
  (|CallParentFunction OtherActor) ; This node is disabled and will not be called.\nDrag off pins to build functionality.
)

(event EventTick
  (params (DeltaSeconds :type Float%20%28single-precision%29))
  (|CallParentFunction DeltaSeconds) ; This node is disabled and will not be called.\nDrag off pins to build functionality.
)

(fn ConstructionScript
  (|CallParentFunction))