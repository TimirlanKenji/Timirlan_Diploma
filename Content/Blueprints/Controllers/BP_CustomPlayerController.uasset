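; Player controller that routes movement, jump, crouch, main action and interaction input to the cached BP_PlayerCharacter.
; An InputAbilityCheck macro gates most input on a valid, living character and a closed menu, though Use skips it.
; Each tick, the character turns toward the cursor hit when the mouse moves horizontally, otherwise toward the right-stick direction.
; The MainMenu action toggles pause, cursor events and the BP_HUD menu.
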(event EventBeginPlay
  (Cofigure|UpdateCurrentPlayerCharacter)
  (CallFunction|UpdateCurrentHUD))

(event EventTick
  (params (DeltaSeconds :type Float%20%28single-precision%29))
  (Utilities|InputAbilityCheck
    (:True
      (if (CallFunction|MouseRotationCheck)
        (Inputs|UpdateRotationbyMouse) ; ..and move there.
        (else
          (Inputs|UpdateRotationbyController))))))

(event Input|ActionEvents|InputActionCrouchDown
  (params (Key :type Key%20Structure :default "None"))
  (:Pressed
    (Utilities|InputAbilityCheck
      (:True
        (Default|Crouching (Variables|Cofigure|GetCurrentPlayerCharacter) true))))
  (:Released
    (Utilities|InputAbilityCheck
      (:True
        (Default|Crouching (Variables|Cofigure|GetCurrentPlayerCharacter) false)))))

(event Input|ActionEvents|InputActionActionMain
  (params (Key :type Key%20Structure :default "None"))
  (:Pressed
    (Utilities|InputAbilityCheck
      (:True
        (Default|ActionMain (Variables|Cofigure|GetCurrentPlayerCharacter) true))))
  (:Released
    (Utilities|InputAbilityCheck
      (:True
        (Default|ActionMain (Variables|Cofigure|GetCurrentPlayerCharacter) false)))))

(event Input|ActionEvents|InputActionJump
  (params (Key :type Key%20Structure :default "None"))
  (:Pressed
    (Utilities|InputAbilityCheck
      (:True
        (Default|Jumping (Variables|Cofigure|GetCurrentPlayerCharacter) true))))
  (:Released
    (Utilities|InputAbilityCheck
      (:True
        (Default|Jumping (Variables|Cofigure|GetCurrentPlayerCharacter) false)))))

(event Input|ActionEvents|InputActionUse
  (params (Key :type Key%20Structure :default "None"))
  (:Pressed
    (Utilities|IsValid (Variables|/Game/Blueprints/Characters/BP_BaseCharacter.BP_BaseCharacter_C|GetCustomActor (Variables|Cofigure|GetCurrentPlayerCharacter))
      (:Is%20Valid
        (bind _success (Default|Interact (Variables|/Game/Blueprints/Characters/BP_BaseCharacter.BP_BaseCharacter_C|GetCustomActor (Variables|Cofigure|GetCurrentPlayerCharacter))))
        (if _success
          (CallFunction|CustomPrintString (Utilities|String|Append (Utilities|GetDisplayName (Variables|/Game/Blueprints/Characters/BP_BaseCharacter.BP_BaseCharacter_C|GetCustomActor (Variables|Cofigure|GetCurrentPlayerCharacter))) "" "Use Successful") true false "(R=0.145529,G=0.911458,B=0.137741,A=1.000000)" 5.0)
          (else
            (CallFunction|CustomPrintString (Utilities|String|Append (Utilities|GetDisplayName (Variables|/Game/Blueprints/Characters/BP_BaseCharacter.BP_BaseCharacter_C|GetCustomActor (Variables|Cofigure|GetCurrentPlayerCharacter))) "" "Use Unsuccessful") true false "(R=0.916667,G=0.156487,B=0.882560,A=1.000000)" 5.0))))
      (:Is%20Not%20Valid
        (CallFunction|CustomPrintString "Actor Not Valid" true false "(R=1.000000,G=0.000000,B=0.023098,A=1.000000)" 5.0)))))

(event Input|ActionEvents|InputActionMainMenu
  (params (Key :type Key%20Structure :default "None"))
  (:Pressed
    (CallFunction|UpdateCurrentHUD)
    (CallFunction|UpdateGamePauseState)
    (Default|ToggleMenu (Variables|Default|GetCurrentHUD) (Variables|Default|GetMenuEnabled) (select (Variables|Default|GetMenuEnabled) "NewEnumerator0" "NewEnumerator1"))))

(event Input|AxisEvents|InputAxisMoveForward
  (params (AxisValue :type Float%20%28single-precision%29))
  ;[1 1 1] Movemet Imput
  (Variables|Inputs|SetAxisMoveForwardValue AxisValue)
  (Utilities|InputAbilityCheck
    (:True
      (Pawn|Input|AddMovementInput (Variables|Cofigure|GetCurrentPlayerCharacter) (Math|Vector|GetForwardVector (Pawn|GetControlRotation (Variables|Cofigure|GetCurrentPlayerCharacter) :!class /Script/Engine.Pawn)) (Variables|Inputs|GetAxisMoveForwardValue) false))))

(event Input|AxisEvents|InputAxisMoveRight
  (params (AxisValue :type Float%20%28single-precision%29))
  ;[1 1 1] Movemet Imput
  (Variables|Inputs|SetAxisMoveRightValue AxisValue)
  (Utilities|InputAbilityCheck
    (:True
      (Pawn|Input|AddMovementInput (Variables|Cofigure|GetCurrentPlayerCharacter) (Math|Vector|GetRightVector (Pawn|GetControlRotation (Variables|Cofigure|GetCurrentPlayerCharacter) :!class /Script/Engine.Pawn)) (Variables|Inputs|GetAxisMoveRightValue) false))))

(fn ConstructionScript)

(fn UpdateRotationbyMouse
  (bind (_hitresult _returnvalue) (Game|Player|GetHitResultUnderCursorbyChannel "TraceTypeQuery1" true))
  (bind _currentplayercharacter (Variables|Cofigure|GetCurrentPlayerCharacter))
  (bind _returnvalue_2 (Transformation|GetActorLocation _currentplayercharacter))
  (bind _location (Collision|BreakHitResult _hitresult))
  (bind _returnvalue_3 (Math|Rotator|FindLookatRotation _returnvalue_2 _location))
  (bind (_roll _pitch _yaw) (Math|Rotator|BreakRotator _returnvalue_3))
  (if _returnvalue
    (Variables|Inputs|SetNewRotation (Math|Rotator|MakeRotator _roll 0.0 _yaw))
    (Transformation|SetActorRotation (Variables|Cofigure|GetCurrentPlayerCharacter) (Variables|Inputs|GetNewRotation))))

(fn UpdateCurrentPlayerCharacter
  (bind _asbp_player_character (Utilities|Casting|CastToBP_PlayerCharacter (Game|Player|GetPlayerPawn 0)))
  (Variables|Cofigure|SetCurrentPlayerCharacter _asbp_player_character))

(fn UpdateRotationbyController
  (LocalVariables|SetL_RightStick (Math|Vector|MakeVector (Input|AxisValues|GetFireForward) (Input|AxisValues|GetFireRight) 0.0))
  (if (> (Math|Vector|VectorLength (LocalVariables|GetL_RightStick)) 0.5)
    (Variables|Inputs|SetNewRotation (Math|Conversions|RotationFromXVector (LocalVariables|GetL_RightStick))))
  (Transformation|SetActorRotation (Variables|Cofigure|GetCurrentPlayerCharacter) (Variables|Inputs|GetNewRotation)))

(fn MouseRotationCheck
  (bind _output_get (Variables|Default|SetControlledByMouse (Math|Vector|NotEqual(Vector) (Math|Vector2D|MakeVector2D (.DeltaX (Class|PlayerController|GetInputMouseDelta)) 0.0) "(X=0.000000,Y=0.000000)" 0.02)))
  (return _output_get))

(fn UpdateCurrentHUD
  (Variables|Default|GetCurrentHUD
    (:then)
    (:else
      (bind _asbp_hud (Utilities|Casting|CastToBP_HUD (HUD|GetHUD)))
      (Variables|Default|SetCurrentHUD _asbp_hud))))

(fn UpdateGamePauseState
  (Variables|Default|SetMenuEnabled (not (Variables|/Game/Blueprints/HUD/BP_HUD.BP_HUD_C|GetIsMenuOpen (Variables|Default|GetCurrentHUD))))
  (Game|SetGamePaused (Variables|Default|GetMenuEnabled))
  (Variables|Default|SetbShowMouseCursor (Variables|Default|GetMenuEnabled))
  (Variables|Default|SetbEnableClickEvents (Variables|Default|GetMenuEnabled))
  (Variables|Default|SetbEnableMouseOverEvents (Variables|Default|GetMenuEnabled)))