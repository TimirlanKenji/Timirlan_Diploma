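; Projectile impact effect actor: a static mesh with adjustable emissive glow that shrinks or fades by curve, then destroys itself.
; BeginPlay creates a dynamic material and starts a disappearance delay timer, presumably triggering StartToDisappear.
; While in progress, Tick samples a float curve to drive EmissiveMult and scale until TimeTarget.
; Scale multiplies the current value each frame, so it compounds and depends on frame rate.
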(event EventBeginPlay
  (bind _staticmesh (Variables|Default|GetStaticMesh))
  (Utilities|Time|SetTimerbyEvent (EventDispatchers|CreateEvent :!event StarttoDisappear) (Variables|Default|GetTimeBeforeDisappear))
  (bind _returnvalue (Rendering|Material|CreateDynamicMaterialInstance _staticmesh 0 (Rendering|Material|GetMaterial _staticmesh 0) "None" :!class /Script/Engine.PrimitiveComponent))
  (Variables|Default|SetDynMat _returnvalue)
  (Rendering|Material|SetScalarParameterValue (Variables|Default|GetDynMat) "EmissiveMult" (Variables|Default|GetEmissive) :!class /Script/Engine.MaterialInstanceDynamic))

(event Collision|EventActorBeginOverlap
  (params (OtherActor :type Actor%20Object%20Reference)))

(event EventTick
  (params (DeltaSeconds :type Float%20%28single-precision%29))
  (Variables|Default|SetTick DeltaSeconds)
  (if (Variables|Default|GetIsInProgress)
    (CallFunction|ScalebyCurveinTick)))

(fn ConstructionScript)

(fn StarttoDisappear
  (Variables|Default|SetIsInProgress true))

(fn ScalebyCurveinTick
  (LocalVariables|SetL_Value (Math|Curves|GetFloatValue (Variables|Default|GetCurve) (Variables|Default|GetTimeCurrent)))
  (Transformation|SetWorldScale3D (Variables|Default|GetStaticMesh) (* (Transformation|GetWorldScale (Variables|Default|GetStaticMesh)) (LocalVariables|GetL_Value)))
  (Rendering|Material|SetScalarParameterValue (Variables|Default|GetDynMat) "EmissiveMult" (* (Variables|Default|GetEmissive) (LocalVariables|GetL_Value)) :!class /Script/Engine.MaterialInstanceDynamic)
  (Variables|Default|SetTimeCurrent (+ (Variables|Default|GetTick) (Variables|Default|GetTimeCurrent)))
  (if (>= (Variables|Default|GetTimeCurrent) (Variables|Default|GetTimeTarget))
    (Variables|Default|SetIsInProgress false)
    (Actor|DestroyActor)))