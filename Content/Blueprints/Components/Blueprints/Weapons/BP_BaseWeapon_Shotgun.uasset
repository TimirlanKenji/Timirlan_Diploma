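; Shotgun weapon Blueprint that fires a horizontal fan of pellets for each shot.
; The SingleShot event calls ShotgunSingeShot, which loops over MaxBulletsInShot to spawn BP_BaseProjectile_ShotgunBullet actors at the Muzzle and pass each CurrentDamage.
; Each pellet's yaw is offset by ShotAngle steps around the muzzle direction, giving an even spread with no randomness.
; It then plays ShotSound once and attaches a spawned BP_MuzzleFX to the Muzzle.
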(event EventBeginPlay
  (|CallParentFunction) ; This node is disabled and will not be called.\nDrag off pins to build functionality.
)

(event Collision|EventActorBeginOverlap
  (params (OtherActor :type Actor%20Object%20Reference))
  (|CallParentFunction OtherActor) ; This node is disabled and will not be called.\nDrag off pins to build functionality.
)

(event EventTick
  (params (DeltaSeconds :type Float%20%28single-precision%29))
  (|CallParentFunction DeltaSeconds) ; This node is disabled and will not be called.\nDrag off pins to build functionality.
)

(event EventSingleShot
  (CallFunction|ShotgunSingeShot))

(fn ConstructionScript
  (|CallParentFunction))

(fn ShotgunSingeShot
  (bind _muzzle (Variables|Default|GetMuzzle))
  (bind _returnvalue (Transformation|GetWorldTransform _muzzle))
  (bind (_roll _pitch _yaw) (Math|Rotator|BreakRotator (.rotation _returnvalue)))
  (Utilities|FlowControl|Sequence
    (:then_0
      (for _index (range 0 (Variables|Default|GetMaxBulletsInShot))
        (LocalVariables|SetL_Indx _index)
        (bind _returnvalue_2 (Game|SpawnActorfromClass "/Game/Blueprints/Weapons/Projectiles/BP_BaseProjectile_ShotgunBullet.BP_BaseProjectile_ShotgunBullet_C" (Math|Transform|MakeTransform (.location _returnvalue) (Math|Rotator|MakeRotator _roll _pitch (+ _yaw (* (Math|Conversions|ToFloat(Integer) (- (LocalVariables|GetL_Indx) (/ (Variables|Default|GetMaxBulletsInShot) 2))) (Variables|Default|GetShotAngle)))) (.scale _returnvalue)) "AdjustIfPossibleButAlwaysSpawn" 0 0))
        (Default|AddDamage _returnvalue_2 (Variables|Default|GetCurrentDamage))))
    (:then_1
      (Audio|Components|Audio|Play (Variables|Default|GetShotSound) 0.0)
      (bind _returnvalue_3 (Game|SpawnActorfromClass "/Game/Blueprints/Weapons/Projectiles/BP_MuzzleFX.BP_MuzzleFX_C" (Transformation|GetWorldTransform (Variables|Default|GetMuzzle)) "Undefined" 0 0))
      (Transformation|AttachComponentToComponent _returnvalue_3 (Variables|Default|GetMuzzle) "None" "SnapToTarget" "SnapToTarget" "SnapToTarget" true))))