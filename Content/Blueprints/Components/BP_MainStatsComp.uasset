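; Stats component that tracks HP, EP shield and death for characters and custom actors.
; On BeginPlay it loads the owner's DT_AllStats row, sets character walk speed, and fills both pools or restores the player's saved values.
; Damage type decides routing: Piercing bypasses EP, while Elemental hits EP double and bare HP at half, with no overflow into HP.
; Dispatchers broadcast configuration, stat changes from damage or capped refills, and death.
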(event EventBeginPlay
  (CallFunction|ConfigureStats))

(event EventTick
  (params (DeltaSeconds :type Float%20%28single-precision%29)))

(fn ReceiveDamage
  (params (InDamage :type Integer) (InType :type ENUM_DamageType%20Enum :default "NewEnumerator0"))
  (LocalVariables|SetL_Damage InDamage)
  (LocalVariables|SetL_Type InType)
  (if (not (Variables|Default|GetIsDead))
    (if (> (Variables|Default|GetCurrentEP) 0)
      (switch Utilities|FlowControl|Switch|SwitchonENUM_DamageType (LocalVariables|GetL_Type)
        (:NewEnumerator0
          (Variables|Default|SetCurrentEP (- (Variables|Default|GetCurrentEP) (LocalVariables|GetL_Damage)))
          (if (> (Variables|Default|GetCurrentEP) 0) :!label _label
            _
            (else
              (Variables|Default|SetCurrentEP 0)))
          (Variables|Default|SetIsDead false))
        (:NewEnumerator1
          (Variables|Default|SetCurrentEP (- (Variables|Default|GetCurrentEP) (* (LocalVariables|GetL_Damage) 2)))
          (goto _label))
        (:NewEnumerator2
          (Variables|Default|SetCurrentHP (- (Variables|Default|GetCurrentHP) (LocalVariables|GetL_Damage)) :!label _label_2)
          (if (> (Variables|Default|GetCurrentHP) 0) :!label _label_3
            (Variables|Default|SetIsDead false)
            (else
              (Variables|Default|SetCurrentHP 0)
              (Variables|Default|SetIsDead true)))))
      (else
        (switch Utilities|FlowControl|Switch|SwitchonENUM_DamageType (LocalVariables|GetL_Type)
          (:NewEnumerator0
            (goto _label_2))
          (:NewEnumerator1
            (Variables|Default|SetCurrentHP (- (Variables|Default|GetCurrentHP) (/ (LocalVariables|GetL_Damage) 2)))
            (goto _label_3))
          (:NewEnumerator2
            (goto _label_2)))))
    (Development|PrintText (Utilities|Text|FormatText "{Actor} | HP {hp} | EP {ep}" (Utilities|Text|ToText(String) (Utilities|GetObjectName (Components|GetOwner))) (Variables|Default|GetCurrentHP) (Variables|Default|GetCurrentEP)) false false (select (Variables|Default|GetIsDead) "(R=1.000000,G=0.000000,B=0.000000,A=1.000000)" "(R=0.062534,G=0.703125,B=0.000000,A=1.000000)") 5.0)
    (Default|CallOnCurrentStatsUpdated (Variables|Default|GetCurrentHP) (Variables|Default|GetCurrentEP) (Variables|Default|GetIsDead) true)
    (if (Variables|Default|GetIsDead)
      (Default|CallOnDied))))

(fn ConfigureStats
  (bind _asbp_base_character (Utilities|Casting|CastToBP_BaseCharacter (Components|GetOwner))
    (:then
      (Variables|Default|SetCurrentCharacter _asbp_base_character)
      (LocalVariables|SetL_RowName (Variables|/Game/Blueprints/Characters/BP_BaseCharacter.BP_BaseCharacter_C|GetCharacterRowName (Variables|Default|GetCurrentCharacter)))
      (LocalVariables|SetL_IsItCharacter true))
    (:CastFailed
      (bind _asbp_custom_actor (Utilities|Casting|CastToBP_CustomActor (Components|GetOwner)))
      (Variables|Default|SetCurrentCustomActor _asbp_custom_actor)
      (LocalVariables|SetL_RowName (Variables|/Game/Blueprints/BP_CustomActor.BP_CustomActor_C|GetCustomActorRowName (Variables|Default|GetCurrentCustomActor)))
      (LocalVariables|SetL_IsItCharacter false)))
  (if (Utilities|Name|NotEqual(Name) (LocalVariables|GetL_RowName) "None")
    (bind _returnvalue (Utilities|GetDataTableRow "/Game/DataTables/DT_AllStats.DT_AllStats" (LocalVariables|GetL_RowName))
      (:then
        (Variables|Default|SetMainStats _returnvalue)
        (if (LocalVariables|GetL_IsItCharacter)
          (CallFunction|ConfigureMovement)
          (Utilities|Casting|CastToBP_PlayerCharacter (Variables|Default|GetCurrentCharacter)
            (:then
              ;[0.1927 0.1927 0.1927] Checks Save Game data related to HP and EP
              (bind _asbp_custom_game_instance (Utilities|Casting|CastToBP_CustomGameInstance (Game|GetGameInstance))
                (:then
                  (if (Variables|/Game/Blueprints/BP_CustomGameInstance.BP_CustomGameInstance_C|GetIsItNewGame _asbp_custom_game_instance)
                    (CallFunction|HealUp true :!label _label)
                    (CallFunction|ShieldUp true)
                    (else
                      (Utilities|IsValid (Variables|/Game/Blueprints/BP_CustomGameInstance.BP_CustomGameInstance_C|GetSaveGameObj _asbp_custom_game_instance)
                        (:Is%20Valid
                          (LocalVariables|SetL_SaveGameObj (Variables|/Game/Blueprints/BP_CustomGameInstance.BP_CustomGameInstance_C|GetSaveGameObj _asbp_custom_game_instance))
                          (Variables|Default|SetCurrentHP (Variables|/Game/Blueprints/BP_SaveGame.BP_SaveGame_C|GetCurrentPlayerHP (LocalVariables|GetL_SaveGameObj)))
                          (Variables|Default|SetCurrentEP (Variables|/Game/Blueprints/BP_SaveGame.BP_SaveGame_C|GetCurrentPlayerEP (LocalVariables|GetL_SaveGameObj)))
                          (Default|CallOnCurrentStatsUpdated (Variables|Default|GetCurrentHP) (Variables|Default|GetCurrentEP) (Variables|Default|GetIsDead) false))
                        (:Is%20Not%20Valid
                          (goto _label))))))
                (:CastFailed
                  (goto _label))))
            (:CastFailed
              (goto _label)))
          (else
            (goto _label)))
        (Default|CallOnConfigureStats))
      (:RowNotFound
        (Development|PrintString "No Such Data Row Name" true true "(R=1.000000,G=0.000000,B=0.166800,A=1.000000)" 5.0)))
    (else
      (Development|PrintString "Has No Any Row Name" true true "(R=1.000000,G=0.000000,B=0.166800,A=1.000000)" 5.0))))

(fn ConfigureMovement
  (Variables|/Script/Engine.CharacterMovementComponent|SetMaxWalkSpeed (Variables|/Script/Engine.Character|GetCharacterMovement (Variables|Default|GetCurrentCharacter)) (.MaxWalkSpeed (Utilities|Struct|BreakSTRUCT_MainStats (Variables|Default|GetMainStats)))))

(fn HealUp
  (params (ToMaximum :type Boolean) (AddHP :type Integer))
  (if ToMaximum
    (Variables|Default|SetCurrentHP (.MaxHP (Utilities|Struct|BreakSTRUCT_MainStats (Variables|Default|GetMainStats))))
    (else
      (LocalVariables|SetL_HP AddHP)
      (Variables|Default|SetCurrentHP (Math|Integer|Min(Integer) (+ (Variables|Default|GetCurrentHP) (LocalVariables|GetL_HP)) (.MaxHP (Utilities|Struct|BreakSTRUCT_MainStats (Variables|Default|GetMainStats)))))))
  (Default|CallOnCurrentStatsUpdated (Variables|Default|GetCurrentHP) (Variables|Default|GetCurrentEP) (Variables|Default|GetIsDead) false))

(fn ShieldUp
  (params (ToMaximum :type Boolean) (AddEP :type Integer))
  (if ToMaximum
    (Variables|Default|SetCurrentEP (.MaxEP (Utilities|Struct|BreakSTRUCT_MainStats (Variables|Default|GetMainStats))))
    (else
      (LocalVariables|SetL_EP AddEP)
      (Variables|Default|SetCurrentEP (Math|Integer|Min(Integer) (+ (Variables|Default|GetCurrentEP) (LocalVariables|GetL_EP)) (.MaxEP (Utilities|Struct|BreakSTRUCT_MainStats (Variables|Default|GetMainStats)))))))
  (Default|CallOnCurrentStatsUpdated (Variables|Default|GetCurrentHP) (Variables|Default|GetCurrentEP) (Variables|Default|GetIsDead) false))

(fn CheckHP
  (return (== (Variables|Default|GetCurrentHP) (.MaxHP (Utilities|Struct|BreakSTRUCT_MainStats (Variables|Default|GetMainStats))))))

(fn CheckEP
  (return (== (Variables|Default|GetCurrentEP) (.MaxEP (Utilities|Struct|BreakSTRUCT_MainStats (Variables|Default|GetMainStats))))))