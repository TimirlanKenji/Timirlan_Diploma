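; Base character Blueprint that provides interaction, crouch, jump and main-action state handling.
; UpdateCustomActor stores a target actor, and pressing E calls Interact on it, printing color-coded debug results for success, failure or an invalid actor.
; Crouching, Jumping and ActionMain turn boolean input into movement calls or button-state flags, with Tick printing while the main action is held.
; BeginPlay calls Binds, which is empty here.
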(event EventBeginPlay
  (CallFunction|Binds))

(event Collision|EventActorBeginOverlap
  (params (OtherActor :type Actor%20Object%20Reference)))

(event EventTick
  (params (DeltaSeconds :type Float%20%28single-precision%29))
  (if (Variables|Default|GetActionMainPressed)
    (Development|PrintString (Utilities|String|Append (Utilities|GetObjectName self) "" "ActionMain Pressed") true false "(R=0.311520,G=0.065224,B=1.000000,A=1.000000)" (Utilities|Time|GetWorldDeltaSeconds))))

(event Input|KeyboardEvents|E
  (params (Key :type Key%20Structure :default "None"))
  (:Pressed
    (Variables|Default|GetCustomActor
      (:then
        (bind _success (Default|Interact (Variables|Default|GetCustomActor)))
        (if _success
          (CallFunction|CustomPrintString (Utilities|String|Append (Utilities|GetDisplayName (Variables|Default|GetCustomActor)) "" "Use Successful") true false "(R=0.145529,G=0.911458,B=0.137741,A=1.000000)" 5.0)
          (else
            (CallFunction|CustomPrintString (Utilities|String|Append (Utilities|GetDisplayName (Variables|Default|GetCustomActor)) "" "Use Unsuccessful") true false "(R=0.916667,G=0.156487,B=0.882560,A=1.000000)" 5.0))))
      (:else
        (CallFunction|CustomPrintString "Actor Not Valid" true false "(R=1.000000,G=0.000000,B=0.023098,A=1.000000)" 5.0)))))

(fn ConstructionScript)

(fn UpdateCustomActor
  (params (InCustomActor :type BP%20Custom%20Actor%20Object%20Reference))
  (Variables|Default|SetCustomActor InCustomActor))

(fn Crouching
  (params (InCrouch :type Boolean))
  (if InCrouch
    (Character|Crouch)
    (Variables|Default|SetCrouch%20Button%20Down true)
    (else
      (Character|UnCrouch)
      (Variables|Default|SetCrouch%20Button%20Down false))))

(fn Jumping
  (params (InJump :type Boolean))
  (if InJump
    (Character|Jump)
    (Variables|Default|SetJump%20Button%20Down (Character|CanJump))
    (else
      (Character|StopJumping)
      (Variables|Default|SetJump%20Button%20Down false))))

(fn Binds)

(fn ActionMain
  (params (IsPressed :type Boolean))
  (Variables|Default|SetActionMainPressed IsPressed))