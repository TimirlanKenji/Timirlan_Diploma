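; Base NPC character Blueprint with overhead-style health and shield bar widgets and pawn sensing.
; On BeginPlay it binds both bars to itself, hiding the shield bar when the stats component's max EP is zero.
; Each tick it rotates the LoockAtCamera component toward the player camera.
; PawnSensing see and hear events are re-broadcast through the NPC's own OnSeePawn and OnHearNoise calls.
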(event OnSeePawn(PawnSensing)
  (params (Pawn :type Pawn%20Object%20Reference))
  (Default|CallOnSeePawn Pawn))

(event OnHearNoise(PawnSensing)
  (params (Instigator :type Pawn%20Object%20Reference) (Location :type Vector%20%28by%20ref%29 :default "0, 0, 0") (Volume :type Float%20%28single-precision%29))
  (Default|CallOnHearNoise Instigator Location Volume))

(event EventBeginPlay
  (|CallParentFunction)
  (CallFunction|WidgetsConfigure))

(event Collision|EventActorBeginOverlap
  (params (OtherActor :type Actor%20Object%20Reference))
  (|CallParentFunction OtherActor) ; This node is disabled and will not be called.\nDrag off pins to build functionality.
)

(event EventTick
  (params (DeltaSeconds :type Float%20%28single-precision%29))
  (|CallParentFunction DeltaSeconds)
  (CallFunction|LookatCamera))

(fn ConstructionScript
  (|CallParentFunction))

(fn LookatCamera
  (Utilities|IsValid (Game|GetPlayerCameraManager 0)
    (:Is%20Valid
      (LocalVariables|SetL_CameraLocation (Camera|GetCameraLocation (Game|GetPlayerCameraManager 0)))
      (Transformation|SetWorldRotation (Variables|Default|GetLoockAtCamera) (Math|Rotator|FindLookatRotation (Transformation|GetWorldLocation (Variables|Default|GetLoockAtCamera)) (LocalVariables|GetL_CameraLocation)) false false))))

(fn WidgetsConfigure
  (Utilities|FlowControl|Sequence
    (:then_0
      (bind _asw_health_bar (Utilities|Casting|CastToW_HealthBar (UserInterface|GetUserWidgetObject (Variables|Default|GetWidgetHP))))
      (Default|UpdateCurrentCharforHP _asw_health_bar self))
    (:then_1
      (if (!= (.MaxEP (Utilities|Struct|BreakSTRUCT_MainStats (Variables|/Game/Blueprints/Components/BP_MainStatsComp.BP_MainStatsComp_C|GetMainStats (Variables|Default|GetBP_MainStatsComp)))) 0)
        (bind _asw_shield_bar (Utilities|Casting|CastToW_ShieldBar (UserInterface|GetUserWidgetObject (Variables|Default|GetWidgetEP))))
        (Default|UpdateCurrentCharforEP _asw_shield_bar self)
        (else
          (Rendering|SetVisibility (Variables|Default|GetWidgetEP) false false))))))